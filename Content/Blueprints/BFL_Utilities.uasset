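; Blueprint function library of shared gameplay helpers.
; GetPlayerCharacter casts player 0's character to BP_PlayerCaracterFP and returns it with a Found flag.
; UpdateBar rounds a current and max value and joins them into "current/max" text for bar displays.
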(fn `GetPlayerCharacter`
  (returns (BP_PlayerCharacterFP :type "/Game/Blueprints/Controllers/BP_PlayerCaracterFP Object Reference") (Found :type Boolean))
  (bind _asbp_player_caracter_fp (cast `/Game/Blueprints/Controllers/BP_PlayerCaracterFP` (`GameplayStatics.GetPlayerCharacter` null))
    (:`then`
      (return _asbp_player_caracter_fp true))
    (:`CastFailed`
      (return null false))))

(fn `UpdateBar`
  (params (Current :type "Float (double-precision)") (Max :type "Float (double-precision)"))
  (returns (ReturnValue :type Text))
  (return (`KismetTextLibrary.Conv_StringToText` (`KismetStringLibrary.Concat_StrStr` (`KismetStringLibrary.Conv_Int64ToString` (`KismetMathLibrary.Round64` Current)) " / " (`KismetStringLibrary.Conv_Int64ToString` (`KismetMathLibrary.Round64` Max))))))